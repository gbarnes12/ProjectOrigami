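; Player Blueprint that builds an orb path spline around itself and handles the pause menu.
; On BeginPlay it rebuilds OrbPath from four points at 100-degree steps, offset by Radius around the actor's up axis and raised above it.
; Escape toggles the pause widget, game pause and mouse cursor.
; The toggle skips the main menu by comparing against a PIE-prefixed level name, which matches only in editor play.
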(event `self.ReceiveBeginPlay`
  (bind _orbpath (`self.OrbPath`))
  (`SplineComponent.ClearSplinePoints` _orbpath)
  ;[1 1 1] Add Spline Points in Radius
  (bind _index (`/Game/Origami/Blueprints/CustomMacro.ForLoopWithStep` 0 360 100)
    (:`LoopBody`
      (`SplineComponent.AddSplinePoint` _orbpath (+ (`self.K2_GetActorLocation`) (`KismetMathLibrary.RotateAngleAxis` (`KismetMathLibrary.MakeVector` (`self.Radius`)) (`KismetMathLibrary.Conv_IntToDouble` _index) (`self.GetActorUpVector`)) (0.0 0.0 100.0)) "World"))
    (:`Completed`
      (`SceneComponent.ResetRelativeTransform` _orbpath)
      (`SceneComponent.K2_SetRelativeLocation` _orbpath (0.0 0.0 0.0) false false))))

(event `InputAction|Escape`
  (params (Key :type "Key Structure" :default "AnyKey"))
  (:`Pressed`
    (`self.TogglePauseMenu`)))

(fn `TogglePauseMenu`
  (bind _ispausemenuactive (`self.IsPauseMenuActive`))
  (bind _pausemenuwidget (`self.PauseMenuWidget`))
  (bind _returnvalue (`self.GetCurrentLevel` self))
  (if (`KismetStringLibrary.NotEqual_StrStr` _returnvalue "UEDPIE_0_MainMenu")
    (bind _output_get (set `self.IsPauseMenuActive` (not _ispausemenuactive)))
    (if _output_get
      (bind _returnvalue_2 (`|CreateWidget` "/Game/Origami/Objects/UI/Hud/Pause/PauseMenuWidget.PauseMenuWidget_C"))
      (bind _output_get_2 (set `self.PauseMenuWidget` _returnvalue_2))
      (`UserWidget.AddToViewport` _output_get_2 0)
      (else
        (`/Engine/EditorBlueprintResources/StandardMacros.IsValid` _pausemenuwidget
          (:`Is Valid`
            (`Widget.RemoveFromParent` _pausemenuwidget)))))
    (bind _returnvalue_3 (`GameplayStatics.SetGamePaused` null _ispausemenuactive))
    (set `PlayerController.bShowMouseCursor` _returnvalue_3 (`GameplayStatics.GetPlayerController` null))))

(fn `UserConstructionScript`)