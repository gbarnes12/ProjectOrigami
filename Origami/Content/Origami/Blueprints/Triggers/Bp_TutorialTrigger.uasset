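; Tutorial trigger actor that shows an image-based tutorial widget on screen when an actor tagged Player overlaps it.
; If ImageToShow is valid, each overlap creates a new TutorialWidget, gives it a reference back to the trigger, sets its image from that texture and adds it to the viewport.
; An optional debug flag draws the collision component's bounds as a box on Tick.
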(event `self.ReceiveActorBeginOverlap`
  (params (OtherActor :type "Actor Object Reference"))
  ;[1 1 1] Create a new Widget whenever we enter the tutorial trigger!
  (set `self.TutorialWidget` null)
  (if (`KismetArrayLibrary.Array_Contains` (`Actor.Tags` OtherActor) "Player")
    (`/Engine/EditorBlueprintResources/StandardMacros.IsValid` (`self.ImageToShow`)
      (:`Is Valid`
        (bind _returnvalue (`|CreateWidget` "/Game/Origami/Objects/UI/Hud/Tutorial/TutorialWidget.TutorialWidget_C"))
        (set `/Game/Origami/Objects/UI/Hud/Tutorial/TutorialWidget.CalledTrigger` self _returnvalue)
        (bind _output_get (set `self.TutorialWidget` _returnvalue))
        (bind _astutorial_widget (cast `/Game/Origami/Objects/UI/Hud/Tutorial/TutorialWidget` _output_get))
        (`Image.SetBrush` (`/Game/Origami/Objects/UI/Hud/Tutorial/TutorialWidget.TutorialImage` _astutorial_widget) (`WidgetBlueprintLibrary.MakeBrushFromTexture` (`self.ImageToShow`)))
        (`UserWidget.AddToViewport` _returnvalue 0)))))

(event `self.ReceiveTick`
  (params (DeltaSeconds :type "Float (single-precision)"))
  (bind (_origin _boxextent) (`KismetSystemLibrary.GetComponentBounds` (`self.CollisionComponent`)))
  ;[1 1 1] Render Debug Box
  (if (`self.ActivateDebugRender`)
    (`KismetSystemLibrary.DrawDebugBox` _origin _boxextent (struct :`R` 1.0 :`B` 0.287649 :`A` 1.0) (struct) 1.0)))

(fn `UserConstructionScript`)