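; Gami Blueprint that toggles the pause menu when the Escape input action is pressed.
; TogglePauseMenu skips the main menu by matching its play-in-editor level name, then creates or removes the pause widget and sets game pause to match.
; Mouse cursor visibility follows the success value returned by SetGamePaused, not the menu state.
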(event `InputAction|Escape`
  (:`Pressed`
    (`self.TogglePauseMenu`)))

(fn `TogglePauseMenu`
  (bind _ispausemenuactive (`self.IsPauseMenuActive`))
  (bind _pausemenuwidget (`self.PauseMenuWidget`))
  (bind _returnvalue (`self.GetCurrentLevel` self))
  (if (`KismetStringLibrary.NotEqual_StrStr` _returnvalue "UEDPIE_0_MainMenu")
    (bind _output_get (set `self.IsPauseMenuActive` (not _ispausemenuactive)))
    (if _output_get
      (bind _returnvalue_2 (`|CreateWidget` "/Game/Origami/Widgets/HUD/PauseMenuWidget.PauseMenuWidget_C"))
      (bind _output_get_2 (set `self.PauseMenuWidget` _returnvalue_2))
      (`UserWidget.AddToViewport` _output_get_2 0)
      (else
        (`/Engine/EditorBlueprintResources/StandardMacros.IsValid` _pausemenuwidget
          (:`Is Valid`
            (`Widget.RemoveFromParent` _pausemenuwidget)))))
    (bind _returnvalue_3 (`GameplayStatics.SetGamePaused` null _ispausemenuactive))
    (set `PlayerController.bShowMouseCursor` _returnvalue_3 (`GameplayStatics.GetPlayerController` null))))

(fn `UserConstructionScript`)